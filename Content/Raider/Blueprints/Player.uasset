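; Player Blueprint that manages health, its HUD bar and the game-over state.
; BeginPlay creates the HealthBar widget, and Tick calls UpdateHealth, which regenerates Hp by RegenRate scaled by delta time and updates the bar's percentage.
; At zero Hp, it adds a GameOver widget, disables character input, shows the cursor and pauses the game.
; UpdateHealth's Damage parameter is unused.
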(event EventBeginPlay
  (bind _returnvalue (UserInterface|CreateWidget "/Game/UI/HealthBar.HealthBar_C"))
  (Variables|Default|SetHealthBarWidget _returnvalue)
  (UserInterface|Viewport|AddtoViewport (Variables|Default|GetHealthBarWidget) 0))

(event EventTick
  (params (DeltaSeconds :type Float%20%28single-precision%29))
  (CallFunction|UpdateHealth 0.0))

(fn ConstructionScript)

(fn UpdateHealth
  (params (Damage :type Float%20%28single-precision%29))
  (bind _returnvalue (Game|GetPlayerController 0))
  ;[1 1 1] UpdateHealth: Custom graph to update the player health slowly and call game over if it reaches 0
  (if (<= (Variables|Default|GetHp) 0.0)
    (bind _returnvalue_2 (UserInterface|CreateWidget "/Game/Raider/Menus/GameOver.GameOver_C"))
    (UserInterface|Viewport|AddtoViewport _returnvalue_2 0)
    (Input|DisableInput (Game|GetPlayerCharacter 0) _returnvalue)
    (Variables|/Script/Engine.PlayerController|SetbShowMouseCursor _returnvalue true)
    (Game|SetGamePaused true)
    (elif (<= (Variables|Default|GetHp) (Variables|Default|GetMaxHp))
      (Variables|Default|SetHp (+ (Variables|Default|GetHp) (* (Utilities|Time|GetWorldDeltaSeconds) (Variables|Default|GetRegenRate))))
      (Variables|/Game/UI/HealthBar.HealthBar_C|SetHealthPercentage (Variables|Default|GetHealthBarWidget) (/ (Variables|Default|GetHp) (Variables|Default|GetMaxHp))))))